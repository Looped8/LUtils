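; Example actor that demonstrates an L-prefixed debug utility library: execution timers, leveled and keyed log messages, loop helpers and debug vector drawing.
; BeginPlay times a delay and a timer event, prints each message level, then runs a delayed loop and a sequential loop that increments ArrayTest, advancing manually.
; Tick rotates VectorA, draws vectors on the actor and player, and logs the flattened camera direction's angle to VectorA.
; GetDebugMask returns a fixed bitmask.
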(event `self.ReceiveBeginPlay`
  (bind _arraytest (`self.ArrayTest`))
  (`|ExecutionSequence`
    (:`then_0`
      ;[1 1 1] Execution timers
      (`/LUtils/BPFL_LDebug.LStartExecutionTimer` "test1")
      (`KismetSystemLibrary.Delay` 5.0)
      (`/LUtils/BPFL_LDebug.LStopExecutionTimer` "test1" true))
    (:`then_1`
      (`/LUtils/BPFL_LDebug.LStartExecutionTimer` "test2")
      (`KismetSystemLibrary.K2_SetTimerDelegate` (delegate `OnTest2Done`) 3.0))
    (:`then_2`
      (`|ExecutionSequence`
        (:`then_0`
          ;[1 1 1] Prints
          (`/LUtils/BPFL_LDebug.LInfo` (`|FormatText` "Info Msg {position}" (`KismetStringLibrary.Conv_VectorToString` (`self.K2_GetActorLocation`))) "Abc" 5.0 (struct :`R` 1.0 :`G` 1.0 :`B` 1.0 :`A` 1.0) true)
          (`/LUtils/BPFL_LDebug.LDebug` "Debug Msg" "None" 8.0 (struct :`R` 1.0 :`B` 0.6 :`A` 1.0) true))
        (:`then_1`
          (`/LUtils/BPFL_LDebug.LSuccess` "Success Msg")
          (`/LUtils/BPFL_LDebug.LWarn` "Warn Msg"))
        (:`then_2`
          (`/LUtils/BPFL_LDebug.LError` "Error Msg"))
        (:`then_3`
          (`|ExecutionSequence`
            (:`then_0`
              ;[1 1 1] ForLoopWithDelay
              (bind _index (`/LUtils/BPML_LUtils.LForLoopWithDelay` 0 4 5.0)
                (:`LoopBody`
                  (`/LUtils/BPFL_LDebug.LDebug` (`KismetTextLibrary.Conv_IntToText` _index)))))
            (:`then_1`
              ;[1 1 1] ForLoopSequential
              (bind _index_2 (`/LUtils/BPML_LUtils.LForLoopSequential` 0 (- (`KismetArrayLibrary.Array_Length` (`self.ArrayTest`)) 1) :!label _label)
                (:`LoopBody`
                  (`KismetArrayLibrary.Array_Set` _arraytest _index_2 (+ (`|GetArrayItem` _arraytest _index_2) 1))
                  (`/LUtils/BPFL_LDebug.LInfo` "Waiting 1s..." "None" 0.5 (struct :`R` 1.0 :`G` 1.0 :`B` 1.0 :`A` 1.0) true)
                  (`KismetSystemLibrary.Delay` 1.0)
                  (goto _label :!via `Next`))
                (:`Completed`
                  (`KismetSystemLibrary.PrintString` "Done"))))))))))

(event `OnTest2Done`
  ;[1 1 1] Execution timers
  (`/LUtils/BPFL_LDebug.LStopExecutionTimer` "test2" true))

(event `self.ReceiveTick`
  (params (DeltaSeconds :type "Float (single-precision)"))
  (bind (_returnvalue_x _returnvalue_y) (`KismetMathLibrary.BreakVector` (`KismetMathLibrary.GetForwardVector` (`Pawn.GetControlRotation` (`GameplayStatics.GetPlayerCharacter` 0)))))
  (bind _returnvalue (`KismetMathLibrary.MakeVector` _returnvalue_x _returnvalue_y))
  (`|ExecutionSequence`
    (:`then_0`
      (`/LUtils/BPFL_LDebug.LDrawDebugVectorOnActor` self (`KismetMathLibrary.Normal` (`KismetMathLibrary.MakeVector` 0.0 1.0 1.0)) (struct :`G` 0.244665 :`B` 1.0 :`A` 1.0) 0.0 5.0 200.0))
    (:`then_1`
      (`SceneComponent.K2_AddRelativeRotation` (`self.VectorA`) (struct :`Yaw` 0.1) false false)
      (`/LUtils/BPFL_LDebug.LDrawDebugVectorOnPlayer` _returnvalue (struct :`R` 1.0 :`G` 0.655376 :`A` 1.0) 0.0 20.0 200.0 (0.0 0.0 80.0) true)
      (`/LUtils/BPFL_LDebug.LDebug` (`KismetTextLibrary.Conv_VectorToText` _returnvalue) "VectorCameraForward")
      (`/LUtils/BPFL_LDebug.LDebug` (`|FormatText` "Angle between camera andred arrow: {ang}°" (`/LUtils/BPFL_LQuickLibrary.GetAngleFromVectors` (`SceneComponent.GetForwardVector` (`self.VectorA`)) _returnvalue)) "AngleACamera")
      (`/LUtils/BPFL_LDebug.LDrawDebugVectorOnActor` self (`/LUtils/BPFL_LQuickLibrary.GetRightVectorFromForwardAndWorldUp` (`SceneComponent.GetForwardVector` (`self.VectorA`))) (struct :`G` 1.0 :`B` 0.362509 :`A` 1.0) 0.0 5.0 100.0 (0.0 0.0 100.0) true))))

(fn `GetDebugMask`
  (returns (Mask :type Integer))
  (return (`|BitmaskLiteral` 30)))

(fn `UserConstructionScript`)